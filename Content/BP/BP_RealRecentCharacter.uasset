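; Mario player character with a wearable Koopa-hat punch mode, a boomerang cap throw, crouching and HP.
; Wearing the hat runs chained timelines that extend glove arms; punches alternate sides, Tick lerps arms back to ready.
; Cursor-hit interface checks plus glove overlaps damage Koopa (BP_Turret) or destroy enemy balls.
; Damage updates the HP widget, knocks back, blocks input, grants blinking invulnerability; death fades out and reloads ThunderLevel.
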(event `self.ReceiveBeginPlay`
  (bind (_returnvalue_location _returnvalue_rotation) (`KismetMathLibrary.BreakTransform` (`SceneComponent.K2_GetComponentToWorld` (`self.CupaHat`))))
  (bind _returnvalue (`|CreateWidget` "/Game/UI/MarioHp.MarioHp_C" (`GameplayStatics.GetPlayerController` 0)))
  (bind _output_get (set `self.UI_MarioHp` _returnvalue))
  (`UserWidget.AddToViewport` _output_get 0)
  (set `PlayerController.bShowMouseCursor` true (`GameplayStatics.GetPlayerController` 0))
  (`SceneComponent.SetVisibility` (`self.CupaHat`) false false)
  (`SceneComponent.SetVisibility` (`self.RA_Root`) false false)
  (`SceneComponent.SetVisibility` (`self.RA_Joint1`) false false)
  (`SceneComponent.SetVisibility` (`self.RA_Sphere1`) false false)
  (`SceneComponent.SetVisibility` (`self.RA_Joint2`) false false)
  (`SceneComponent.SetVisibility` (`self.RA_Gold`) false false)
  (`SceneComponent.SetVisibility` (`self.RightGlove`) false false)
  (`SceneComponent.SetVisibility` (`self.LA_Root`) false false)
  (`SceneComponent.SetVisibility` (`self.LA_Joint1`) false false)
  (`SceneComponent.SetVisibility` (`self.LA_Sphere1`) false false)
  (`SceneComponent.SetVisibility` (`self.LA_Joint2`) false false)
  (`SceneComponent.SetVisibility` (`self.LA_Gold`) false false)
  (`SceneComponent.SetVisibility` (`self.LeftGlove`) false false)
  (bind _outactors (`GameplayStatics.GetAllActorsOfClass` "/Game/KOOPA/Blueprints/BP_WhiteHat.BP_WhiteHat_C"))
  (set `self.PunchCapVar` (`|GetArrayItem` _outactors))
  (bind _outactors_2 (`GameplayStatics.GetAllActorsOfClass` "/Game/KOOPA/Blueprints/BP_Turret.BP_Turret_C"))
  (set `self.TurretVar` (`|GetArrayItem` _outactors_2))
  (bind _outactors_3 (`GameplayStatics.GetAllActorsOfClass` "/Game/MARIOs/BP/BP_EnemyBall.BP_EnemyBall_C"))
  (set `self.EnemyBallVar` (`|GetArrayItem` _outactors_3))
  (`KismetSystemLibrary.Delay` 3.0)
  ;[1 1 1] 쿠파 밀려나면 쓰고 있던 펀치 캡 벗겨짐
  (`SceneComponent.SetVisibility` (`self.CupaHat`) false false)
  (`SceneComponent.SetVisibility` (`self.RA_Root`) false false)
  (`SceneComponent.SetVisibility` (`self.RA_Joint1`) false false)
  (`SceneComponent.SetVisibility` (`self.RA_Sphere1`) false false)
  (`SceneComponent.SetVisibility` (`self.RA_Joint2`) false false)
  (`SceneComponent.SetVisibility` (`self.RA_Gold`) false false)
  (`SceneComponent.SetVisibility` (`self.RightGlove`) false false)
  (`SceneComponent.SetVisibility` (`self.LA_Root`) false false)
  (`SceneComponent.SetVisibility` (`self.LA_Joint1`) false false)
  (`SceneComponent.SetVisibility` (`self.LA_Sphere1`) false false)
  (`SceneComponent.SetVisibility` (`self.LA_Joint2`) false false)
  (`SceneComponent.SetVisibility` (`self.LA_Gold`) false false)
  (`SceneComponent.SetVisibility` (`self.LeftGlove`) false false)
  (`|SpawnActorFromClass` "/Game/KOOPA/Blueprints/BP_DestroyingWhiteHat.BP_DestroyingWhiteHat_C" (`KismetMathLibrary.MakeTransform` _returnvalue_location _returnvalue_rotation (0.5 0.5 0.5)) "Undefined" "MultiplyWithRoot" null null) ; 쿠파모자 위치에 생성해서 모자 벗겨지는 척함
  (`KismetSystemLibrary.PrintString` "spawn white hat")
  (set `self.CanDestroyHat` true)
  (set `self.CanPunching` false) ; 모자 벗겨지면 펀치 불가
)

(event `EnhancedInput|/Game/ThirdPerson/Input/Actions/IA_WearHat`
  (params (ActionValue :type Boolean) (ElapsedSeconds :type "Float (double-precision)") (TriggeredSeconds :type "Float (double-precision)") (InputAction :type "InputAction Object Reference" :default "/Game/ThirdPerson/Input/Actions/IA_WearHat.IA_WearHat"))
  (bind (_relativescale3d_x _relativescale3d_y) (`KismetMathLibrary.BreakVector` (`SceneComponent.RelativeScale3D` (`self.LA_Root`))))
  (bind (_relativescale3d_x_2 _relativescale3d_y_2) (`KismetMathLibrary.BreakVector` (`SceneComponent.RelativeScale3D` (`self.RA_Root`))))
  ;[1 1 1] 모자 쓰기
  (:`Started`
    (set `self.canWearHat` false)
    (`SceneComponent.SetVisibility` (`self.CupaHat`) true false)
    (set `self.canThrow` false)
    (set `self.CanPunching` true)
    (bind (_direction _wear) (`Timeline|Timeline` :!via `PlayFromStart`) ; 애니메이션 작업 시 애니메이션으로 대체
      (:`Update`
        (`SceneComponent.K2_SetRelativeLocation` (`self.CupaHat`) (`KismetMathLibrary.MakeVector` 0.0 0.0 _wear) false false))
      (:`Finished`
        (`SceneComponent.SetVisibility` (`self.CupaHat`) true false)
        (`SceneComponent.SetVisibility` (`self.RA_Root`) true false)
        (`SceneComponent.SetVisibility` (`self.RA_Joint1`) true false)
        (`SceneComponent.SetVisibility` (`self.RA_Sphere1`) true false)
        (`SceneComponent.SetVisibility` (`self.RA_Joint2`) true false)
        (`SceneComponent.SetVisibility` (`self.RA_Gold`) true false)
        (`SceneComponent.SetVisibility` (`self.RightGlove`) true false)
        (`SceneComponent.SetVisibility` (`self.LA_Root`) true false)
        (`SceneComponent.SetVisibility` (`self.LA_Joint1`) true false)
        (`SceneComponent.SetVisibility` (`self.LA_Sphere1`) true false)
        (`SceneComponent.SetVisibility` (`self.LA_Joint2`) true false)
        (`SceneComponent.SetVisibility` (`self.LA_Gold`) true false)
        (`SceneComponent.SetVisibility` (`self.LeftGlove`) true false)
        (`KismetSystemLibrary.PrintString` "모자 써서 펀치상태 완료")
        (bind (_direction_2 _glovez) (`Timeline|GloveArmScale` :!via `PlayFromStart`) ; 팔 나오기
          (:`Update`
            (`SceneComponent.SetRelativeScale3D` (`self.RA_Root`) (`KismetMathLibrary.MakeVector` _relativescale3d_x_2 _relativescale3d_y_2 _glovez))
            (`SceneComponent.SetRelativeScale3D` (`self.LA_Root`) (`KismetMathLibrary.MakeVector` _relativescale3d_x _relativescale3d_y _glovez)))
          (:`Finished`
            (`|ExecutionSequence`
              (:`then_0`
                (bind (_direction_3 _ra_root _ra_spherex _ra_spherez) (`Timeline|RA_PunchReady` :!via `PlayFromStart`) ; 펀치 준비 장전
                  (:`Update`
                    (`SceneComponent.K2_SetRelativeRotation` (`self.RA_Root`) (`KismetMathLibrary.MakeRotator` 0.0 _ra_root) false false)
                    (`SceneComponent.K2_SetRelativeRotation` (`self.RA_Sphere1`) (`KismetMathLibrary.MakeRotator` _ra_spherex 0.0 _ra_spherez) false false)
                    (`SceneComponent.K2_SetRelativeRotation` (`self.LA_Sphere1`) (`KismetMathLibrary.MakeRotator` _ra_spherex 0.0 (* _ra_spherez -1.0)) false false))))
              (:`then_1`
                (bind (_direction_4 _la_root) (`Timeline|LA_PunchReady` :!via `PlayFromStart`)
                  (:`Update`
                    (`SceneComponent.K2_SetRelativeRotation` (`self.LA_Root`) (`KismetMathLibrary.MakeRotator` 0.0 _la_root) false false))
                  (:`Finished`
                    (`|ExecutionSequence`
                      (:`then_0`
                        (bind (_direction_5 _ra_root_x _ra_root_y _ra_sphere_x _ra_sphere_z _la_root_y) (`Timeline|RALA_PunchReadyFin` :!via `PlayFromStart`)
                          (:`Update`
                            (`SceneComponent.K2_SetRelativeRotation` (`self.RA_Root`) (`KismetMathLibrary.MakeRotator` _ra_root_x _ra_root_y) false false)
                            (`SceneComponent.K2_SetRelativeRotation` (`self.RA_Sphere1`) (`KismetMathLibrary.MakeRotator` _ra_sphere_x 0.0 _ra_sphere_z) false false)
                            (`SceneComponent.K2_SetRelativeRotation` (`self.LA_Root`) (`KismetMathLibrary.MakeRotator` (* _ra_root_x -1.0) _la_root_y) false false)
                            (`SceneComponent.K2_SetRelativeRotation` (`self.LA_Sphere1`) (`KismetMathLibrary.MakeRotator` _ra_sphere_x 0.0 (* _ra_sphere_z -1.0)) false false))
                          (:`Finished`
                            ;[1 1 1] 펀치 준비완료했을때의 회전값 미리 저장
                            (set `self.RA_RootFinRot` (`SceneComponent.RelativeRotation` (`self.RA_Root`)))
                            (set `self.RA_SphereFinRot` (`SceneComponent.RelativeRotation` (`self.RA_Sphere1`)))
                            (set `self.LA_RootFinRot` (`SceneComponent.RelativeRotation` (`self.LA_Root`)))
                            (set `self.LA_SphereFinRot` (`SceneComponent.RelativeRotation` (`self.LA_Sphere1`)))))))))))))))))

(event `DestroyCupaHatLocUpdate`
  (bind _hatbackloc (`self.hatBackLoc`))
  (bind _relativelocation (`SceneComponent.RelativeLocation` (`self.CupaHat`)))
  (`KismetArrayLibrary.Array_Set` _hatbackloc 0 _relativelocation)
  (`KismetArrayLibrary.Array_Set` _hatbackloc 1 (+ _relativelocation (* (`self.GetActorForwardVector`) 150.0) (* (`self.GetActorUpVector`) 150.0)))
  (set `self.destroyHat` true))

(event `EnhancedInput|/Game/ThirdPerson/Input/Actions/IA_Punch`
  (params (ActionValue :type Boolean) (ElapsedSeconds :type "Float (double-precision)") (TriggeredSeconds :type "Float (double-precision)") (InputAction :type "InputAction Object Reference" :default "/Game/ThirdPerson/Input/Actions/IA_Punch.IA_Punch"))
  (bind _turretvar (`self.TurretVar`))
  (bind _hitresult (`PlayerController.GetHitResultUnderCursorForObjects` (`GameplayStatics.GetPlayerController` 0) (`|MakeArray` "ObjectTypeQuery2" :!type "EObjectTypeQuery Enum") true))
  ;[1 1 1] 마리오가 Cupa Hat을 썼고, 쿠파와 충돌해있고, 쿠파를 클릭했고, Glove가 쿠파한테 닿았으면 펀치 가능
  (:`Started`
    (if (`self.CanPunching`)
      (`/Engine/EditorBlueprintResources/StandardMacros.FlipFlop`
        (:`A`
          (`self.PlayAnimMontage` "/Game/MARIOs/Animations/Anim_Sequences/Mario_PunchLeft_Montage.Mario_PunchLeft_Montage")
          (`self.RA_Punch_LA_Stay`))
        (:`B`
          (`self.PlayAnimMontage` "/Game/MARIOs/Animations/Anim_Sequences/Mario_PunchRight_Montage.Mario_PunchRight_Montage") ; 펀치 애니메이션
          (`self.LA_Punch_RA_Stay`)))
      (if (`self.isCupaAlive`)
        (if (and (`KismetSystemLibrary.DoesImplementInterface` (`.HitActor` (`GameplayStatics.BreakHitResult` _hitresult)) "/Game/MARIOs/Interface/CupaAttack.CupaAttack_C") (or (`PrimitiveComponent.IsOverlappingComponent` (`self.RightGlove`) (`/Game/KOOPA/Blueprints/BP_Turret.CupaCollision` (`self.TurretVar`))) (`PrimitiveComponent.IsOverlappingComponent` (`self.LeftGlove`) (`/Game/KOOPA/Blueprints/BP_Turret.CupaCollision` (`self.TurretVar`)))))
          (if (`/Game/KOOPA/Blueprints/BP_Turret.isOverlappingCupa` (`self.TurretVar`))
            (`KismetSystemLibrary.PrintString` "쿠파 앞")
            (`KismetSystemLibrary.PrintString` "쿠파 공격")
            (`KismetSystemLibrary.PrintString` (`KismetSystemLibrary.GetDisplayName` (`.HitActor` (`GameplayStatics.BreakHitResult` _hitresult))))
            (`/Game/KOOPA/Blueprints/BP_Turret.Damage` _turretvar)
            (if (== (`CppTurret.KoopaHealth` _turretvar) 5)
              _))
          (else
            (`KismetSystemLibrary.PrintString` "쿠파 아님")
            (if (and (`KismetSystemLibrary.DoesImplementInterface` (`.HitActor` (`GameplayStatics.BreakHitResult` _hitresult)) "/Game/MARIOs/Interface/BallDestructable.BallDestructable_C") (or (`PrimitiveComponent.IsOverlappingComponent` (`self.RightGlove`) (`/Game/MARIOs/BP/BP_EnemyBall.EnemyBallColl` (`self.EnemyBallVar`))) (`PrimitiveComponent.IsOverlappingComponent` (`self.LeftGlove`) (`/Game/MARIOs/BP/BP_EnemyBall.EnemyBallColl` (`self.EnemyBallVar`)))))
              (`KismetSystemLibrary.PrintString` "can destruct ball")
              (`/Game/MARIOs/BP/BP_EnemyBall.Destruct Ball` (`self.EnemyBallVar`)))))
        (else
          (`KismetSystemLibrary.PrintString` "쿠파 die")))
      (else
        (`KismetSystemLibrary.PrintString` "모자 먼저 쓰세요")))))

(event `RA_Punch_LA_Stay`
  (bind (_ra_rootfinrot_roll _ra_rootfinrot_pitch) (`KismetMathLibrary.BreakRotator` (`self.RA_RootFinRot`)))
  ;[1 1 1] 펀치 회전값 조절
  (`SceneComponent.K2_SetRelativeRotation` (`self.RA_Root`) (`KismetMathLibrary.MakeRotator` 50.0 _ra_rootfinrot_pitch) false false)
  (`SceneComponent.K2_SetRelativeRotation` (`self.RA_Sphere1`) (`KismetMathLibrary.MakeRotator` 65.0) false false)
  (`SceneComponent.K2_SetRelativeRotation` (`self.LA_Root`) (`self.LA_RootFinRot`) false false)
  (`SceneComponent.K2_SetRelativeRotation` (`self.LA_Sphere1`) (`self.LA_SphereFinRot`) false false)
  (set `self.RA_RootPunchRot` (`SceneComponent.RelativeRotation` (`self.RA_Root`)))
  (set `self.RA_SpherePunchRot` (`SceneComponent.RelativeRotation` (`self.RA_Sphere1`)))
  (set `self.bRA_Return` true))

(event `LA_Punch_RA_Stay`
  ;[1 1 1] 펀치 회전값 조절
  (`SceneComponent.K2_SetRelativeRotation` (`self.LA_Root`) (`KismetMathLibrary.MakeRotator` -50.0 120.0) false false)
  (`SceneComponent.K2_SetRelativeRotation` (`self.LA_Sphere1`) (`KismetMathLibrary.MakeRotator` 65.0) false false)
  (`SceneComponent.K2_SetRelativeRotation` (`self.RA_Root`) (`self.RA_RootFinRot`) false false)
  (`SceneComponent.K2_SetRelativeRotation` (`self.RA_Sphere1`) (`self.RA_SphereFinRot`) false false)
  (set `self.LA_RootPunchRot` (`SceneComponent.RelativeRotation` (`self.LA_Root`)))
  (set `self.LA_SpherePunchRot` (`SceneComponent.RelativeRotation` (`self.LA_Sphere1`)))
  (set `self.bLA_Return` true))

(event `EnhancedInput|/Game/ThirdPerson/Input/Actions/IA_CapBoomerang`
  (params (ActionValue :type Boolean) (ElapsedSeconds :type "Float (double-precision)") (TriggeredSeconds :type "Float (double-precision)") (InputAction :type "InputAction Object Reference" :default "/Game/ThirdPerson/Input/Actions/IA_CapBoomerang.IA_CapBoomerang"))
  (bind (_returnvalue_location _returnvalue_rotation _returnvalue_scale) (`KismetMathLibrary.BreakTransform` (`SceneComponent.K2_GetComponentToWorld` (`self.Arrow1`))))
  ;[1 1 1] 모자 날리기
  (:`Started`
    (if (`self.canThrow`)
      (if (`self.isOnMario`)
        (`self.PlayAnimMontage` "/Game/MARIOs/Animations/Anim_Sequences/Mario_Throw_Montage.Mario_Throw_Montage")
        (set `self.isOnMario` false) ; 모자 날렸으면 다시 못 날리게
        (bind _returnvalue (`|SpawnActorFromClass` "/Game/BP/BP_MarioThrowingCap.BP_MarioThrowingCap_C" (`KismetMathLibrary.MakeTransform` (+ _returnvalue_location (0.0 0.0 10.0)) _returnvalue_rotation _returnvalue_scale) "Undefined" "MultiplyWithRoot" null null))
        (set `self.MarioCapSpawned` _returnvalue)
        (bind (_direction _newtrack_1) (`Timeline|MarioSpin` :!via `PlayFromStart`)
          (:`Update`
            (`SceneComponent.K2_SetRelativeRotation` (`self.Mesh`) (`KismetMathLibrary.MakeRotator` 0.0 0.0 _newtrack_1) false false)
            (`SceneComponent.SetVisibility` (`self.Cap`) false false)
            (`KismetSystemLibrary.Delay` 1.0)
            (`/Game/BP/BP_MarioThrowingCap.ReturnToPlayer` (`self.MarioCapSpawned`))
            (set `self.isOnMario` true) ; 모자 return됐으면 다시 날릴 수 있게
          )))
      (else
        (`KismetSystemLibrary.PrintString` "펀치캡 쓴 상태에서는 못 날림")))))

(event `self.ReceiveTick`
  (params (DeltaSeconds :type "Float (single-precision)"))
  (if (`self.bRA_Return`)
    (bind _output_get (set `self.RA_lerpAlphaValue` (`KismetMathLibrary.FClamp` (+ (`self.RA_lerpAlphaValue`) 0.05))))
    (`|ExecutionSequence`
      (:`then_0`
        (`SceneComponent.K2_SetRelativeRotation` (`self.RA_Root`) (`KismetMathLibrary.RLerp` (`self.RA_RootPunchRot`) (`self.RA_RootFinRot`) _output_get true) false false))
      (:`then_1`
        (`SceneComponent.K2_SetRelativeRotation` (`self.RA_Sphere1`) (`KismetMathLibrary.RLerp` (`self.RA_SpherePunchRot`) (`self.RA_SphereFinRot`) _output_get true) false false)))
    (if (>= (`self.RA_lerpAlphaValue`) 1.0)
      (`KismetSystemLibrary.Delay` 0.2)
      (set `self.bRA_Return` false)
      (set `self.RA_lerpAlphaValue` 0.0))
    (elif (`self.bLA_Return`)
      (bind _output_get_2 (set `self.LA_lerpAlphaValue` (`KismetMathLibrary.FClamp` (+ (`self.LA_lerpAlphaValue`) 0.05))))
      (`|ExecutionSequence`
        (:`then_0`
          (`SceneComponent.K2_SetRelativeRotation` (`self.LA_Root`) (`KismetMathLibrary.RLerp` (`self.LA_RootPunchRot`) (`self.LA_RootFinRot`) _output_get_2 true) false false))
        (:`then_1`
          (`SceneComponent.K2_SetRelativeRotation` (`self.LA_Sphere1`) (`KismetMathLibrary.RLerp` (`self.LA_SpherePunchRot`) (`self.LA_SphereFinRot`) _output_get_2 true) false false)))
      (if (>= (`self.LA_lerpAlphaValue`) 1.0)
        (`KismetSystemLibrary.Delay` 0.2)
        (set `self.bLA_Return` false)
        (set `self.LA_lerpAlphaValue` 0.0)))))

(event `self.ReceiveAnyDamage`
  (params (Damage :type "Float (single-precision)") (DamageType :type "DamageType Object Reference") (InstigatedBy :type "Controller Object Reference") (DamageCauser :type "Actor Object Reference"))
  (bind (_returnvalue_x _returnvalue_y _returnvalue_z) (`KismetMathLibrary.BreakVector` (`SceneComponent.GetForwardVector` (`self.CameraBoom`))))
  (bind (_returnvalue_x_2 _returnvalue_y_2 _returnvalue_z_2) (`KismetMathLibrary.BreakVector` (* (`self.GetActorForwardVector` (`GameplayStatics.GetPlayerCharacter` 0)) -1000.0)))
  ;[1 1 1] 마리오 데미지
  (if (`self.isMarioDamaged`)
    (`|ExecutionSequence`
      (:`then_0`
        (`self.PlayAnimMontage` "/Game/MARIOs/Animations/Anim_Sequences/Mario_Damage_Montage.Mario_Damage_Montage"))
      (:`then_1`
        (`self.LaunchCharacter` (`KismetMathLibrary.MakeVector` _returnvalue_x_2 _returnvalue_y_2 (+ _returnvalue_z_2 250.0))) ; 뒤로 밀려나기
        (`self.DisableInput` (`GameplayStatics.GetPlayerController` 0)) ; 데미지 입으면 1.5초 동안 모든 행동 block됨
        (bind _output_get (set `self.MarioHp` (`KismetMathLibrary.FClamp` (- (`self.MarioHp`) Damage) 0.0 6.0)))
        (`/Game/UI/MarioHp.MinusHp` (`self.UI_MarioHp`) _output_get)
        (if (== (`self.MarioHp`) 0.0)
          (bind _returnvalue (`PrimitiveComponent.CreateDynamicMaterialInstance` (`self.Plane`) 0 "/Game/UI/M_marioDeathFade.M_marioDeathFade" "None"))
          (`self.K2_SetActorRotation` (`KismetMathLibrary.MakeRotator` 0.0 0.0 _returnvalue_z))
          (bind (_direction _newtrack_0) (`Timeline|Timeline_0` :!via `PlayFromStart`)
            (:`Update`
              (`MaterialInstanceDynamic.SetScalarParameterValue` _returnvalue "Fade" _newtrack_0)
              (set `self.isMarioDamaged` false)
              (`self.DisableInput` (`GameplayStatics.GetPlayerController` 0))
              (`KismetSystemLibrary.Delay` 5.0)
              (`GameplayStatics.OpenLevel` "ThunderLevel") ; 죽었으면 다시 레벨 불러오기
            ))
          (else
            (`|ExecutionSequence`
              (:`then_0`
                (`KismetSystemLibrary.Delay` 1.0)
                (`self.PlayAnimMontage` "/Game/MARIOs/Animations/Anim_Sequences/Mario_Gettingup_Montage.Mario_Gettingup_Montage")
                (`KismetSystemLibrary.Delay` 2.5) ; 데미지 1번 입으면 2.5초 이동 불가
                (`self.EnableInput` (`GameplayStatics.GetPlayerController` 0)))
              (:`then_1`
                (set `self.isMarioDamaged` false) ; 데미지 1번 입으면 4초동안 무적상태
                (`KismetSystemLibrary.Delay` 6.5)
                (set `self.isMarioDamaged` true))))))
      (:`then_2`
        (`KismetSystemLibrary.K2_SetTimerDelegate` (delegate `GGamBBack`) 0.2 true) ; 0.2초마다 실행
      ))))

(event `Heal`
  ;[1 1 1] 마리오 HP 회복
  (bind _output_get (set `self.MarioHp` (`KismetMathLibrary.FClamp` (+ (`self.MarioHp`) 1.0) 0.0 6.0)))
  (`/Game/UI/MarioHp.PlusHp` (`self.UI_MarioHp`) _output_get))

(event `GGamBBack`
  (if (<= (`self.timerCnt`) 25)
    (`SceneComponent.SetVisibility` (`self.Mesh`) false false)
    (`SceneComponent.SetVisibility` (`self.Cap`) false false)
    (`KismetSystemLibrary.Delay` 0.1)
    (`SceneComponent.SetVisibility` (`self.Mesh`) true false)
    (`SceneComponent.SetVisibility` (`self.Cap`) true false)
    (`KismetSystemLibrary.Delay` 0.1)
    (`/Engine/EditorBlueprintResources/StandardMacros.IncrementInt` (`self.timerCnt`))))

(event `EnhancedInput|/Game/ThirdPerson/Input/Actions/IA_Crouch`
  (params (ActionValue :type Boolean) (ElapsedSeconds :type "Float (double-precision)") (TriggeredSeconds :type "Float (double-precision)") (InputAction :type "InputAction Object Reference" :default "/Game/ThirdPerson/Input/Actions/IA_Crouch.IA_Crouch"))
  ;[1 1 1] 웅크리기
  (:`Triggered`
    (set `self.isCrouched` true)
    (bind _asabp_mario (cast `/Game/MARIOs/Animations/Anim_BPs/ABP_Mario` (`SkeletalMeshComponent.GetAnimInstance` (`self.Mesh`)) :!label _label))
    (set `/Game/MARIOs/Animations/Anim_BPs/ABP_Mario.anim_IsCrouched` (`self.isCrouched`) _asabp_mario))
  (:`Completed`
    (set `self.isCrouched` false)
    (goto _label)))

(fn `UserConstructionScript`
  (`SceneComponent.K2_AttachToComponent` (`self.Cap`) (`self.Mesh`) "CapSocket" "KeepRelative" "KeepRelative" "KeepRelative" true))
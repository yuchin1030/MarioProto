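; BP_WhiteHat is a Koopa hat that damages overlapping actors until Mario's thrown cap knocks it loose and makes it wearable.
; The first cap hit turns it toward the player, then Tick moves it along the player's forward and up vectors while spinning.
; After a short delay it descends to a fixed floor height, where a timeline plays a landing scale effect.
; It also flags player overlap; older waypoint-arc logic remains disconnected.
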(event `self.ReceiveBeginPlay`
  (bind (_returnvalue_roll _returnvalue_pitch) (`KismetMathLibrary.BreakRotator` (`self.K2_GetActorRotation`)))
  (`|ExecutionSequence`
    (:`then_0`
      (bind _outactors (`GameplayStatics.GetAllActorsOfClass` "/Game/BP/BP_MarioThrowingCap.BP_MarioThrowingCap_C"))
      (set `self.ThrowCapVar` (`|GetArrayItem` _outactors))
      (set `self.NewRotY` _returnvalue_pitch))
    (:`then_1`
      (bind _outactors_2 (`GameplayStatics.GetAllActorsOfClass` "/Game/BP/BP_RealRecentCharacter.BP_RealRecentCharacter_C"))
      (set `self.CharacterVar` (`|GetArrayItem` _outactors_2)))))

(event `self.boxComp.OnComponentBeginOverlap`
  (params (OverlappedComponent :type "PrimitiveComponent Object Reference") (OtherActor :type "Actor Object Reference") (OtherComp :type "PrimitiveComponent Object Reference") (OtherBodyIndex :type Integer) (bFromSweep :type Boolean) (SweepResult :type "HitResult Structure (by ref)"))
  (bind (_returnvalue_roll _returnvalue_pitch _returnvalue_yaw) (`KismetMathLibrary.BreakRotator` (`KismetMathLibrary.MakeRotFromZX` (`self.GetActorUpVector`) (- (`self.K2_GetActorLocation` (`self.CharacterVar`)) (`self.K2_GetActorLocation`)))))
  (`|ExecutionSequence`
    (:`then_0`
      (if (not (`self.CanWearHat`))
        (`GameplayStatics.ApplyDamage` OtherActor 1.0)))
    (:`then_1`
      (cast `/Game/BP/BP_RealRecentCharacter` OtherActor)
      (set `self.isOverlappingHat` true)
      (`KismetSystemLibrary.PrintString` "yes overlap"))
    (:`then_2`
      (cast `/Game/BP/BP_MarioThrowingCap` OtherActor)
      (`/Engine/EditorBlueprintResources/StandardMacros.DoOnce` false
        (:`Completed`
          (set `self.isThrowingCap` true)
          (set `self.bStopLocWhiteHat` false)
          (set `self.bStopRotWhiteHat` false)
          (`self.K2_SetActorRotation` (`KismetMathLibrary.MakeRotator` _returnvalue_roll _returnvalue_pitch _returnvalue_yaw)))))))

(event `self.boxComp.OnComponentEndOverlap`
  (params (OverlappedComponent :type "PrimitiveComponent Object Reference") (OtherActor :type "Actor Object Reference") (OtherComp :type "PrimitiveComponent Object Reference") (OtherBodyIndex :type Integer))
  (`|ExecutionSequence`
    (:`then_0`
      (cast `/Game/BP/BP_RealRecentCharacter` OtherActor)
      (set `self.isOverlappingHat` false)
      (`KismetSystemLibrary.PrintString` "no overlap"))
    (:`then_1`
      (cast `/Game/BP/BP_MarioThrowingCap` OtherActor)
      (set `self.isThrowingCap` false))))

(event `CupaHatRotate`
  (set `self.StopRot` true)
  (bind (_direction _newtrack_0) (`Timeline|Timeline_2`)
    (:`Update`
      (`self.K2_SetActorRotation` (`KismetMathLibrary.MakeRotator` 0.0 _newtrack_0))
      (set `self.CanWearHat` true)
      (`KismetSystemLibrary.PrintString` "모자 쓸 수 있는 상태 Ready"))))

(event `UpdateInterp`)

(event `self.ReceiveTick`
  (params (DeltaSeconds :type "Float (single-precision)"))
  (bind (_returnvalue_x _returnvalue_y _returnvalue_z) (`KismetMathLibrary.BreakVector` (`self.K2_GetActorLocation`)))
  (bind _speed (`self.speed`))
  (bind _rotatingmovement (`self.RotatingMovement`))
  (bind _returnvalue (+ (`self.K2_GetActorLocation`) (* (`KismetMathLibrary.Normal` (`self.GetActorForwardVector` (`self.CharacterVar`)) 1.0) _speed DeltaSeconds) (* (`KismetMathLibrary.Normal` (`self.GetActorUpVector` (`self.CharacterVar`)) 1.0) _speed DeltaSeconds)))
  (if (not (`self.bStopRotWhiteHat`))
    (set `self.CanWearHat` true)
    (`|ExecutionSequence`
      (:`then_0`
        (if (not (`self.canHatFall`))
          (`self.K2_SetActorLocation` _returnvalue)
          (`KismetSystemLibrary.PrintString` (`KismetStringLibrary.Conv_VectorToString` _returnvalue))
          (`KismetSystemLibrary.Delay` 0.5)
          (set `self.canHatFall` true)))
      (:`then_1`
        (`ActorComponent.Activate` (`self.RotatingMovement`) false))
      (:`then_2`
        (if (`self.canHatFall`)
          (`ActorComponent.Deactivate` (`self.RotatingMovement`))
          (bind _output_get (set `self.Return Value Z` _returnvalue_z))
          (`|ExecutionSequence`
            (:`then_0`
              (bind _returnvalue_2 (`KismetMathLibrary.FClamp` (- _output_get 5.0) 100.0 590.0))
              (`self.K2_SetActorLocation` (`KismetMathLibrary.MakeVector` _returnvalue_x _returnvalue_y _returnvalue_2))
              (if (<= _returnvalue_2 100.0)
                (bind (_direction _newtrack_0) (`Timeline|ArriveFloorHatScale`) ; 땅에 떨어졌을때 떨어진듯한 효과
                  (:`Update`
                    (`self.SetActorScale3D` (`KismetMathLibrary.MakeVector` 1.0 _newtrack_0 1.0))
                    (set `RotatingMovementComponent.RotationRate` (struct :`Yaw` 180.0) _rotatingmovement)
                    (`ActorComponent.Activate` _rotatingmovement false)))))))))))

(fn `UserConstructionScript`)
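; BP_Turret is a Koopa (Cupa) boss actor that fires bullets and can be damaged and killed.
; Twelve seconds after BeginPlay it toggles fire and flame visibility, then spawns three timed BP_Bullets; swingHat replays that volley.
; The Mario component damages overlapping actors, CupaCollision tracks player overlap, and Tick replays the spin montage.
; Damage decrements HP, runs a knockback timeline at a threshold, and at zero destroys the boss and clears the player's IsCupaAlive.
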(event `self.ReceiveBeginPlay`
  (`KismetSystemLibrary.Delay` 12.0)
  (`SceneComponent.ToggleVisibility` (`self.fire8`) false)
  (`SceneComponent.ToggleVisibility` (`self.fire7`) false)
  (`SceneComponent.ToggleVisibility` (`self.fire6`) false)
  (`SceneComponent.ToggleVisibility` (`self.fire1`) false)
  (`SceneComponent.ToggleVisibility` (`self.fire2`) false)
  (`SceneComponent.ToggleVisibility` (`self.fire3`) false)
  (`SceneComponent.ToggleVisibility` (`self.fire4`) false)
  (`SceneComponent.ToggleVisibility` (`self.fire5`) false)
  (`SceneComponent.ToggleVisibility` (`self.flame1`) false)
  (`SceneComponent.ToggleVisibility` (`self.flame2`) false)
  (`SceneComponent.ToggleVisibility` (`self.flame3`) false)
  (`SceneComponent.ToggleVisibility` (`self.flame4`) false)
  (`KismetSystemLibrary.Delay` 3.0 :!label _label)
  (`|SpawnActorFromClass` "/Game/KOOPA/Blueprints/BP_Bullet.BP_Bullet_C" (`SceneComponent.K2_GetComponentToWorld` (`self.Arrow`)) "AdjustIfPossibleButAlwaysSpawn" "MultiplyWithRoot" null null)
  (`KismetSystemLibrary.Delay` 3.0)
  (`|SpawnActorFromClass` "/Game/KOOPA/Blueprints/BP_Bullet.BP_Bullet_C" (`SceneComponent.K2_GetComponentToWorld` (`self.Arrow`)) "AdjustIfPossibleButAlwaysSpawn" "MultiplyWithRoot" null null)
  (`KismetSystemLibrary.Delay` 3.0)
  (`|SpawnActorFromClass` "/Game/KOOPA/Blueprints/BP_Bullet.BP_Bullet_C" (`SceneComponent.K2_GetComponentToWorld` (`self.Arrow`)) "AdjustIfPossibleButAlwaysSpawn" "MultiplyWithRoot" null null)
  (`|PlayMontage` (`self.TurretMesh`) "/Game/KOOPA/SpinAttack/Spin_In_Place1_Montage.Spin_In_Place1_Montage"))

(event `swing Hat`
  (goto _label))

(event `self.ReceiveActorBeginOverlap`
  (params (OtherActor :type "Actor Object Reference")))

(event `self.ReceiveTick`
  (params (DeltaSeconds :type "Float (single-precision)"))
  (`|PlayMontage` (`self.TurretMesh`) "/Game/KOOPA/SpinAttack/Spin_In_Place1_Montage.Spin_In_Place1_Montage"))

(event `self.Mario.OnComponentBeginOverlap`
  (params (OverlappedComponent :type "PrimitiveComponent Object Reference") (OtherActor :type "Actor Object Reference") (OtherComp :type "PrimitiveComponent Object Reference") (OtherBodyIndex :type Integer) (bFromSweep :type Boolean) (SweepResult :type "HitResult Structure (by ref)"))
  (`GameplayStatics.ApplyDamage` OtherActor 1.0))

(event `self.CupaCollision.OnComponentBeginOverlap`
  (params (OverlappedComponent :type "PrimitiveComponent Object Reference") (OtherActor :type "Actor Object Reference") (OtherComp :type "PrimitiveComponent Object Reference") (OtherBodyIndex :type Integer) (bFromSweep :type Boolean) (SweepResult :type "HitResult Structure (by ref)"))
  (cast `/Game/ThirdPerson/Blueprints/BP_ThirdPersonCharacter` OtherActor)
  (set `self.isOverlappingCupa` true)
  (`KismetSystemLibrary.PrintString` "cupa yes overlap"))

(event `self.CupaCollision.OnComponentEndOverlap`
  (params (OverlappedComponent :type "PrimitiveComponent Object Reference") (OtherActor :type "Actor Object Reference") (OtherComp :type "PrimitiveComponent Object Reference") (OtherBodyIndex :type Integer))
  (cast `/Game/ThirdPerson/Blueprints/BP_ThirdPersonCharacter` OtherActor)
  (set `self.isOverlappingCupa` false)
  (`KismetSystemLibrary.PrintString` "cupa no overlap"))

(event `Damage`
  (bind _output_get (set `self.cupaHP` (- (`self.cupaHP`) 1)))
  (`KismetSystemLibrary.PrintString` (`KismetStringLibrary.Conv_IntToString` _output_get))
  (if (== (`self.cupaHP`) 5)
    (bind (_direction _back) (`Timeline|CupaBack`)
      (:`Update`
        (`SceneComponent.K2_SetRelativeLocation` (`self.TurretMesh`) (`KismetMathLibrary.MakeVector` 0.0 _back) false false)))
    (elif (<= (`self.cupaHP`) 0)
      (`self.K2_DestroyActor`)
      (bind _asbp_third_person_character (cast `/Game/ThirdPerson/Blueprints/BP_ThirdPersonCharacter` (`GameplayStatics.GetPlayerCharacter` 0)))
      (set `/Game/ThirdPerson/Blueprints/BP_ThirdPersonCharacter.isCupaAlive` false _asbp_third_person_character))))

(fn `UserConstructionScript`)
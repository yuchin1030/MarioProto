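; Mario's thrown cap projectile, which flies out briefly and can return to the player.
; Tick stops the projectile after a 0.2 second delay, or immediately when the PunchCap's CupaHatCollision overlaps the player's spawned cap, also triggering CupaHatRotate.
; ReturnToPlayer moves the cap once to the character mesh, re-shows the worn cap and destroys the actor.
; Line trace and rotation-stop experiments remain unconnected.
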(event `self.ReceiveBeginPlay`
  (bind _outactors (`GameplayStatics.GetAllActorsOfClass` "/Game/ThirdPerson/Blueprints/BP_ThirdPersonCharacter.BP_ThirdPersonCharacter_C"))
  (set `self.TpcVar` (`|GetArrayItem` _outactors))
  (bind _outactors_2 (`GameplayStatics.GetAllActorsOfClass` "/Game/MARIOs/BP/PunchCap.PunchCap_C"))
  (set `self.PunchCap Var` (`|GetArrayItem` _outactors_2)))

(event `self.ReceiveTick`
  (params (DeltaSeconds :type "Float (single-precision)"))
  (if (`PrimitiveComponent.IsOverlappingActor` (`/Game/MARIOs/BP/PunchCap.CupaHatCollision` (`self.PunchCap Var`)) (`/Game/ThirdPerson/Blueprints/BP_ThirdPersonCharacter.MarioCapSpawned` (`self.TpcVar`)))
    (`MovementComponent.StopMovementImmediately` (`self.ProjectileMovement`)) ; 쿠파가 던진 모자 enemy에 맞으면 그 자리에서 throw stop
    (`/Game/MARIOs/BP/PunchCap.CupaHatRotate` (`self.PunchCap Var`))
    (else
      (`KismetSystemLibrary.Delay` 0.2)
      (`MovementComponent.StopMovementImmediately` (`self.ProjectileMovement`)))))

(event `ReturnToPlayer`
  ;[1 1 1] 모자 날리고 되돌아오기
  (`/Engine/EditorBlueprintResources/StandardMacros.DoOnce` false
    (:`Completed`
      (bind _asbp_third_person_character (cast `/Game/ThirdPerson/Blueprints/BP_ThirdPersonCharacter` (`GameplayStatics.GetPlayerCharacter` 0)))
      (bind (_returnvalue_location _returnvalue_rotation) (`KismetMathLibrary.BreakTransform` (`SceneComponent.K2_GetComponentToWorld` (`Character.Mesh` _asbp_third_person_character))))
      (`KismetSystemLibrary.MoveComponentTo` (`self.DefaultSceneRoot`) _returnvalue_location _returnvalue_rotation)
      (`SceneComponent.SetVisibility` (`/Game/ThirdPerson/Blueprints/BP_ThirdPersonCharacter.Cap` _asbp_third_person_character) true false)
      (`self.K2_DestroyActor`))))

(fn `UserConstructionScript`)